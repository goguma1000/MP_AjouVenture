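; BP_Chito is a character Blueprint that lets the character interact with objects in front of it.
; On the IA_Interaction input, it line-traces a short distance along the capsule's forward vector on TraceTypeQuery3, with timed debug drawing.
; A hit actor implementing the InteractableActor interface receives InteractMessage, keeping interaction decoupled from specific classes.
; An alternative that searches overlapping actors remains in the graph but is disconnected and never runs.
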(event Input|EnhancedActionEvents|EnhancedInputActionIA_Interaction
  (params (ActionValue :type Boolean) (ElapsedSeconds :type Float%20%28double-precision%29) (TriggeredSeconds :type Float%20%28double-precision%29) (InputAction :type Input%20Action%20Object%20Reference :default "/Game/Blueprints/Characters/Input/Actions/IA_Interaction.IA_Interaction"))
  (bind _returnvalue (Transformation|GetActorLocation))
  (:Triggered
    (bind (_outhit _returnvalue_2) (Collision|LineTraceByChannel _returnvalue (+ _returnvalue (* (Math|Vector|GetForwardVector (Variables|Default|GetCapsuleComponent)) 1.5e+02)) "TraceTypeQuery3" false 0 "ForDuration" true "(R=1.000000,G=0.000000,B=0.000000,A=1.000000)" "(R=0.000000,G=1.000000,B=0.000000,A=1.000000)" 2.0))
    (if _returnvalue_2
      (if (Utilities|DoesObjectImplementInterface (.HitActor (Collision|BreakHitResult _outhit)) "/Game/Blueprints/BP_Interface/InteractableActor.InteractableActor_C")
        (Class|InteractableActor|Interact(Message) (.HitActor (Collision|BreakHitResult _outhit)))))))

(event EventBeginPlay)

(event Collision|EventActorBeginOverlap
  (params (OtherActor :type Actor%20Object%20Reference)))

(event EventTick
  (params (DeltaSeconds :type Float%20%28single-precision%29)))

(fn ConstructionScript)