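; BP_Console is an interactable console actor that opens a puzzle board UI.
; A screen-space guide widget, created at BeginPlay, becomes visible while the player's controlled pawn overlaps the actor.
; Interact prints a debug string, hides the guide, swaps the Enhanced Input mapping context from DefaultMappingContext to IMC_Default and adds a new BP_CS_PuzzleBoard widget to the viewport.
; Nothing here restores the previous mapping context.
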(event Custom|Change%20Mapping%20Context
  (bind _returnvalue (Game|GetPlayerController 0))
  (bind _returnvalue_2 (PlayerController|LocalPlayerSubsystems|GetEnhancedInputLocalPlayerSubsystem _returnvalue))
  (Input|RemoveMappingContext _returnvalue_2 "/Game/Blueprints/Characters/Input/DefaultMappingContext.DefaultMappingContext" "(bIgnoreAllPressedKeysUntilRelease=True,bForceImmediately=False,bNotifyUserSettings=False)")
  (Input|AddMappingContext _returnvalue_2 "/Game/ThirdPerson/Input/IMC_Default.IMC_Default" 0 "(bIgnoreAllPressedKeysUntilRelease=True,bForceImmediately=False,bNotifyUserSettings=False)"))

(event EventBeginPlay
  (bind _guide_message (Variables|Default|GetGuide_Message))
  (bind _returnvalue (UserInterface|CreateWidget "/Game/Blueprints/UI/BP_Interaction_GuideMSG.BP_Interaction_GuideMSG_C"))
  (UserInterface|SetWidget _guide_message _returnvalue)
  (Class|WidgetComponent|SetWidgetSpace _guide_message "Screen"))

(event Collision|EventActorBeginOverlap
  (params (OtherActor :type Actor%20Object%20Reference))
  (if (== OtherActor (Pawn|GetControlledPawn (Game|GetPlayerController 0)))
    (Rendering|SetVisibility (Variables|Default|GetGuide_Message) true false)))

(event EventTick
  (params (DeltaSeconds :type Float%20%28single-precision%29)))

(event Collision|EventActorEndOverlap
  (params (OtherActor :type Actor%20Object%20Reference))
  (if (== (Pawn|GetControlledPawn (Game|GetPlayerController 0)) OtherActor)
    (Rendering|SetVisibility (Variables|Default|GetGuide_Message) false false)))

(event EventInteract
  (Development|PrintString "Interact with Chito")
  (CallFunction|ChangeMappingContext)
  (Rendering|SetVisibility (Variables|Default|GetGuide_Message) false false)
  (bind _returnvalue (UserInterface|CreateWidget "/Game/Blueprints/UI/BP_CS_PuzzleBoard.BP_CS_PuzzleBoard_C"))
  (UserInterface|Viewport|AddtoViewport _returnvalue 0))

(fn ConstructionScript)